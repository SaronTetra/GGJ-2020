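; Train waggon actor that rides a looping rail spline, copying the Locomotive's speed when flagged as a wagon.
; Each Tick advances Distance by Speed per frame without delta time, places Front and Back on the spline an Offset apart, and aims FrontPoint away from BackPoint.
; The construction script can preview placement on the rail.
; AddSpeed changes Speed unless broken and tilts the throttle handle to match.
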(event `self.ReceiveTick`
  (params (DeltaSeconds :type "Float (single-precision)"))
  (bind _distance (`self.Distance`))
  (bind _spline (`/Game/GGJ-2020/Track/BP_TrackSplineFixed.Spline` (`self.Rails`)))
  (bind _returnvalue (mod (+ (`self.Distance`) (`self.Offset`)) (`SplineComponent.GetSplineLength` _spline)))
  (`|ExecutionSequence`
    (:`then_0`
      ;[1 1 1] Rotate
      (`SceneComponent.K2_SetWorldRotation` (`self.Front point`) (`KismetMathLibrary.FindLookAtRotation` (`SceneComponent.K2_GetComponentLocation` (`self.Back point`)) (`SceneComponent.K2_GetComponentLocation` (`self.Front point`))) false false))
    (:`then_1`
      (bind _output_get (set `self.Distance` (mod (+ (`self.Distance`) (`self.Speed`)) (`SplineComponent.GetSplineLength` _spline))))
      (`|ExecutionSequence`
        (:`then_1`
          (`SceneComponent.K2_SetWorldLocationAndRotation` (`self.Front`) (`SplineComponent.GetLocationAtDistanceAlongSpline` _spline _distance "World") (`SplineComponent.GetRotationAtDistanceAlongSpline` _spline _distance "World") false false)
          (`SceneComponent.K2_SetWorldLocationAndRotation` (`self.Back`) (`SplineComponent.GetLocationAtDistanceAlongSpline` _spline _returnvalue "World") (`SplineComponent.GetRotationAtDistanceAlongSpline` _spline _returnvalue "World") false false))))
    (:`then_2`
      (if (`self.IsWagoon`)
        (set `self.Speed` (`/Game/GGJ-2020/Train/BP_Train_GGJ.Speed` (`self.Locomotive`)))))))

(event `self.ReceiveBeginPlay`
  (set `self.Distance` (`self.Start Offset`)))

(fn `AddSpeed`
  (params (Amount :type "Float (double-precision)"))
  (bind _speed (`self.Speed`))
  (if (not (`self.IsBroken`))
    (set `self.Speed` (+ Amount (`KismetMathLibrary.FClamp` _speed 0.0 50.0)))
    (`SceneComponent.K2_SetRelativeRotation` (`self.SM_Handle_Throttle`) (`KismetMathLibrary.MakeRotator` 0.0 (+ (`self.MinAngle`) _speed)) false false)))

(fn `UserConstructionScript`
  (bind _returnvalue (+ (`self.Distance`) (`self.Start Offset`)))
  (bind _spline (`/Game/GGJ-2020/Track/BP_TrackSplineFixed.Spline` (`self.Rails`)))
  (bind _returnvalue_2 (mod (+ (`self.Distance`) (`self.Offset`) (`self.Start Offset`)) (`SplineComponent.GetSplineLength` _spline)))
  (if (`self.SpawnOnRail`)
    (`SceneComponent.K2_SetWorldLocationAndRotation` (`self.Front`) (`SplineComponent.GetLocationAtDistanceAlongSpline` _spline _returnvalue "World") (`SplineComponent.GetRotationAtDistanceAlongSpline` _spline _returnvalue "World") false false)
    (`SceneComponent.K2_SetWorldLocationAndRotation` (`self.Back`) (`SplineComponent.GetLocationAtDistanceAlongSpline` _spline _returnvalue_2 "World") (`SplineComponent.GetRotationAtDistanceAlongSpline` _spline _returnvalue_2 "World") false false)
    (`SceneComponent.K2_SetWorldRotation` (`self.Front point`) (`KismetMathLibrary.FindLookAtRotation` (`SceneComponent.K2_GetComponentLocation` (`self.Back point`)) (`SceneComponent.K2_GetComponentLocation` (`self.Front point`))) false false)))