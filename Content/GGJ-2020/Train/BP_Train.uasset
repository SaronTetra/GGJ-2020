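; Train actor that runs endlessly around a looping Rails spline.
; Each tick advances Distance by Speed, wrapped by spline length and not scaled by delta time.
; Front and Back are snapped to the spline's position and rotation at Distance and Distance plus Offset.
; FrontPoint is first rotated along the line from BackPoint to FrontPoint, using their positions before that tick's move.
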(event `self.ReceiveTick`
  (params (DeltaSeconds :type "Float (single-precision)"))
  (bind _distance (`self.Distance`))
  (bind _spline (`/Game/GGJ-2020/Track/BP_Rails.Spline` (`self.Rails`)))
  (bind _returnvalue (mod (+ (`self.Distance`) (`self.Offset`)) (`SplineComponent.GetSplineLength` (`/Game/GGJ-2020/Track/BP_Rails.Spline` (`self.Rails`)))))
  (`|ExecutionSequence`
    (:`then_0`
      ;[1 1 1] Rotate
      (`SceneComponent.K2_SetWorldRotation` (`self.Front point`) (`KismetMathLibrary.FindLookAtRotation` (`SceneComponent.K2_GetComponentLocation` (`self.Back point`)) (`SceneComponent.K2_GetComponentLocation` (`self.Front point`))) false false))
    (:`then_1`
      (bind _output_get (set `self.Distance` (mod (+ (`self.Distance`) (`self.Speed`)) (`SplineComponent.GetSplineLength` _spline))))
      (`|ExecutionSequence`
        (:`then_1`
          (`SceneComponent.K2_SetWorldLocationAndRotation` (`self.Front`) (`SplineComponent.GetLocationAtDistanceAlongSpline` _spline _distance "World") (`SplineComponent.GetRotationAtDistanceAlongSpline` _spline _distance "World") false false)
          (`SceneComponent.K2_SetWorldLocationAndRotation` (`self.Back`) (`SplineComponent.GetLocationAtDistanceAlongSpline` _spline _returnvalue "World") (`SplineComponent.GetRotationAtDistanceAlongSpline` _spline _returnvalue "World") false false))))))

(fn `UserConstructionScript`)