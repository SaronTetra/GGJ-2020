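; Train car for a GGJ 2020 game, usable as locomotive or wagon, that loops along a rail spline.
; Each tick it places front and back points on the spline, aims the body between them and drives audio from speed; wagons copy locomotive speed.
; AddSpeed moves the throttle handle and speed.
; Locomotives randomly break down at stations, and damage events spend game-mode Bolts to repair them.
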(event `self.ReceiveTick`
  (params (DeltaSeconds :type "Float (single-precision)"))
  (bind _distance (`self.Distance`))
  (bind _speed (`self.Speed`))
  (bind _spline (`/Game/GGJ-2020/Track/BP_TrackSplineFixed.Spline` (`self.Rails`)))
  (bind _returnvalue (mod (+ (`self.Distance`) (`self.Offset`)) (`SplineComponent.GetSplineLength` _spline)))
  (bind _returnvalue_2 (* (`KismetMathLibrary.Conv_BoolToDouble` (not (`self.IsBroken`))) 1.0))
  (`|ExecutionSequence`
    (:`then_0`
      ;[1 1 1] Rotate
      (`SceneComponent.K2_SetWorldRotation` (`self.Front point`) (`KismetMathLibrary.FindLookAtRotation` (`SceneComponent.K2_GetComponentLocation` (`self.Back point`)) (`SceneComponent.K2_GetComponentLocation` (`self.Front point`))) false false)
      (`AudioComponent.SetPitchMultiplier` (stale `self.ReceiveBeginPlay` _returnvalue_2) (/ _speed 100.0) :!label _label)
      (`AudioComponent.SetVolumeMultiplier` (stale `self.ReceiveBeginPlay` _returnvalue) _returnvalue_2)
      (`AudioComponent.SetVolumeMultiplier` (stale `self.ReceiveBeginPlay` _returnvalue_2) _returnvalue_2)
      (`AudioComponent.SetPitchMultiplier` (stale `self.ReceiveBeginPlay` _returnvalue) (`KismetMathLibrary.FClamp` (/ _speed 100.0) 0.5 1.5)))
    (:`then_1`
      (bind _output_get (set `self.Distance` (mod (+ (`self.Distance`) (`self.Speed`)) (`SplineComponent.GetSplineLength` _spline))))
      (`|ExecutionSequence`
        (:`then_1`
          (`SceneComponent.K2_SetWorldLocationAndRotation` (`self.Front`) (`SplineComponent.GetLocationAtDistanceAlongSpline` _spline _distance "World") (`SplineComponent.GetRotationAtDistanceAlongSpline` _spline _distance "World") false false)
          (`SceneComponent.K2_SetWorldLocationAndRotation` (`self.Back`) (`SplineComponent.GetLocationAtDistanceAlongSpline` _spline _returnvalue "World") (`SplineComponent.GetRotationAtDistanceAlongSpline` _spline _returnvalue "World") false false))))
    (:`then_2`
      (if (`self.IsWagoon`)
        (set `self.Speed` (`/Game/GGJ-2020/Train/BP_Train_GGJ.Speed` (`self.Locomotive`)))))))

(event `self.ReceiveBeginPlay`
  (set `self.Distance` (`self.Start Offset`))
  (`SceneComponent.K2_SetRelativeRotation` (`self.SM_Handle_Throttle`) (`KismetMathLibrary.MakeRotator` 0.0 (`self.MinAngle`)) false false)
  (bind _returnvalue (`AddComponent|NODE_AddAudioComponent-2`))
  (bind _returnvalue_2 (`AddComponent|NODE_AddAudioComponent-3`))
  (goto _label))

(event `self.ReceiveActorBeginOverlap`
  (params (OtherActor :type "Actor Object Reference"))
  (if (and (== (`GameplayStatics.GetObjectClass` OtherActor) "/Game/GGJ-2020/Train/BP_Station.BP_Station_C") (not (`self.IsWagoon`)))
    (if (> (`KismetMathLibrary.RandomIntegerInRange` 0 100) 50)
      (`GameplayStatics.PlaySoundAtLocation` "/Game/StarterContent/Audio/Explosion02.Explosion02" (`SceneComponent.K2_GetComponentLocation` (`self.Platform`)) (struct) 1.0 1.0 0.0 null null null)
      (`KismetSystemLibrary.PrintString` ":(")
      (set `self.Speed` 0.0)
      (bind _returnvalue (`GameplayStatics.SpawnEmitterAtLocation` "/Game/StarterContent/Particles/P_Smoke.P_Smoke" (`SceneComponent.K2_GetComponentLocation` (`self.Front point`)) (struct) (4.0 4.0 4.0)))
      (set `self.IsBroken` true)
      (`SceneComponent.K2_SetRelativeRotation` (`self.SM_Handle_Throttle`) (`KismetMathLibrary.MakeRotator` 0.0 (`self.MinAngle`)) false false)
      (else
        (`KismetSystemLibrary.PrintString` ":)")))))

(event `self.ReceiveAnyDamage`
  (params (Damage :type "Float (single-precision)") (DamageType :type "DamageType Object Reference") (InstigatedBy :type "Controller Object Reference") (DamageCauser :type "Actor Object Reference"))
  (bind _astrain_points (cast `/Game/GGJ-2020/Core/TrainPoints` (`GameplayStatics.GetGameMode`)))
  (bind _bolts (`/Game/GGJ-2020/Core/TrainPoints.Bolts` _astrain_points))
  (bind _returnvalue (>= _bolts (`self.BoltsRequired`)))
  (if _returnvalue
    (set `/Game/GGJ-2020/Core/TrainPoints.Bolts` (- _bolts 3) _astrain_points)
    (bind _result (`/Engine/EditorBlueprintResources/StandardMacros.IncrementInt` (`self.TrainHealth`))
      (:`  `
        (if (> _result 3)
          (`ActorComponent.K2_DestroyComponent` (stale `self.ReceiveActorBeginOverlap` _returnvalue))
          (set `self.IsBroken` false))))
    (else
      (set `/Game/GGJ-2020/Core/TrainPoints.ShowMessage` (not _returnvalue) _astrain_points)
      (`KismetSystemLibrary.Delay` 1.0)
      (set `/Game/GGJ-2020/Core/TrainPoints.ShowMessage` false _astrain_points))))

(fn `AddSpeed`
  (params (Amount :type "Float (double-precision)"))
  (bind _speed (`self.Speed`))
  (if (not (`self.IsBroken`))
    (set `self.Speed` (+ Amount (`KismetMathLibrary.FClamp` _speed 0.0 150.0)))
    (`SceneComponent.K2_SetRelativeRotation` (`self.SM_Handle_Throttle`) (`KismetMathLibrary.MakeRotator` 0.0 (+ (`self.MinAngle`) _speed)) false false)))

(fn `UserConstructionScript`
  (bind _returnvalue (+ (`self.Distance`) (`self.Start Offset`)))
  (bind _spline (`/Game/GGJ-2020/Track/BP_TrackSplineFixed.Spline` (`self.Rails`)))
  (bind _returnvalue_2 (mod (+ (`self.Distance`) (`self.Offset`) (`self.Start Offset`)) (`SplineComponent.GetSplineLength` _spline)))
  (if (`self.SpawnOnRail`)
    (`SceneComponent.K2_SetWorldLocationAndRotation` (`self.Front`) (`SplineComponent.GetLocationAtDistanceAlongSpline` _spline _returnvalue "World") (`SplineComponent.GetRotationAtDistanceAlongSpline` _spline _returnvalue "World") false false)
    (`SceneComponent.K2_SetWorldLocationAndRotation` (`self.Back`) (`SplineComponent.GetLocationAtDistanceAlongSpline` _spline _returnvalue_2 "World") (`SplineComponent.GetRotationAtDistanceAlongSpline` _spline _returnvalue_2 "World") false false)
    (`SceneComponent.K2_SetWorldRotation` (`self.Front point`) (`KismetMathLibrary.FindLookAtRotation` (`SceneComponent.K2_GetComponentLocation` (`self.Back point`)) (`SceneComponent.K2_GetComponentLocation` (`self.Front point`))) false false)))