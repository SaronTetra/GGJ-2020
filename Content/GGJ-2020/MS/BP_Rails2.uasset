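; BP_Rails2 is a spline-driven rail actor that lays a repeated mesh along an editable spline path.
; The construction script steps along the spline at Spacing intervals, adding and attaching a spline mesh with the chosen Mesh and forward axis for each segment.
; Each segment takes positions and tangents from the spline by distance, with tangent length clamped to Spacing so the pieces deform cleanly.
; The event graph has no active logic.
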(fn `UserConstructionScript`
  (locals (NewLocalVar_0 :type "SplineMeshComponent Object Reference"))
  (bind _spacing (`self.Spacing`))
  (bind _spacing_2 (`self.Spacing`))
  (bind _spline (`self.Spline`))
  (for _index (range (+ (`KismetMathLibrary.FFloor` (/ (`SplineComponent.GetSplineLength` (`self.Spline`)) (`self.Spacing`))) 1))
    (bind _returnvalue (`AddComponent|NODE_AddSplineMeshComponent-2`))
    (`StaticMeshComponent.SetStaticMesh` _returnvalue (`self.Mesh`))
    (`SplineMeshComponent.SetForwardAxis` _returnvalue (`self.Forward Axis`) true)
    (`SceneComponent.K2_AttachToComponent` _returnvalue (`self.Spline`) "None" "KeepRelative" "KeepRelative" "KeepRelative" true)
    (bind _returnvalue_2 (* _index _spacing_2))
    (bind _returnvalue_3 (* (+ _index 1) _spacing_2))
    (`SplineMeshComponent.SetStartAndEnd` _returnvalue (`SplineComponent.GetLocationAtDistanceAlongSpline` _spline _returnvalue_2 "Local") (`KismetMathLibrary.ClampVectorSize` (`SplineComponent.GetTangentAtDistanceAlongSpline` _spline _returnvalue_2 "Local") 0.0 _spacing) (`SplineComponent.GetLocationAtDistanceAlongSpline` _spline _returnvalue_3 "Local") (`KismetMathLibrary.ClampVectorSize` (`SplineComponent.GetTangentAtDistanceAlongSpline` _spline _returnvalue_3 "Local") 0.0 _spacing) true)))