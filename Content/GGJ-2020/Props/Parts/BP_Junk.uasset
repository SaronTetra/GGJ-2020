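; BP_Junk is a collectible junk part that adds one to the Parts count on the TrainPoints game mode when an actor overlaps it, then destroys itself.
; On BeginPlay it picks a random mesh from beam, pipe, spring and gear variants.
; It then sets that mesh's collision to WorldStatic with an overlap response to Pawns.
; The overlap handler does not filter which actor triggers the pickup.
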(event `self.ReceiveActorBeginOverlap`
  (params (OtherActor :type "Actor Object Reference"))
  (bind _astrain_points (cast `/Game/GGJ-2020/Core/TrainPoints` (`GameplayStatics.GetGameMode`)))
  (set `/Game/GGJ-2020/Core/TrainPoints.Parts` (+ (`/Game/GGJ-2020/Core/TrainPoints.Parts` _astrain_points) 1) _astrain_points)
  (`self.K2_DestroyActor`))

(event `self.ReceiveBeginPlay`
  (bind _staticmesh (`self.StaticMesh`))
  (bind _staticmesh_2 (`self.StaticMesh`))
  (`|ExecutionSequence`
    (:`then_0`
      (switch `int` (`KismetMathLibrary.RandomIntegerInRange` 0 5)
        (:`Default`
          (`KismetSystemLibrary.PrintString` "fumck"))
        (:`0`
          (`StaticMeshComponent.SetStaticMesh` _staticmesh "/Game/GGJ-2020/Props/Parts/SM_Junk__Beam.SM_Junk__Beam"))
        (:`1`
          (`StaticMeshComponent.SetStaticMesh` _staticmesh "/Game/GGJ-2020/Props/Parts/SM_Junk__Pipe.SM_Junk__Pipe"))
        (:`2`
          (`StaticMeshComponent.SetStaticMesh` _staticmesh "/Game/GGJ-2020/Props/Parts/SM_Junk__Spring.SM_Junk__Spring"))
        (:`3`
          (`StaticMeshComponent.SetStaticMesh` _staticmesh "/Game/GGJ-2020/Props/Parts/SM_Gear_01.SM_Gear_01"))
        (:`4`
          (`StaticMeshComponent.SetStaticMesh` _staticmesh "/Game/GGJ-2020/Props/Parts/SM_Gear_02.SM_Gear_02"))
        (:`5`
          (`StaticMeshComponent.SetStaticMesh` _staticmesh "/Game/GGJ-2020/Props/Parts/SM_Gear_03.SM_Gear_03"))))
    (:`then_1`
      (`PrimitiveComponent.SetCollisionObjectType` _staticmesh_2 "ECC_WorldStatic")
      (`PrimitiveComponent.SetCollisionResponseToChannel` _staticmesh_2 "ECC_Pawn" "ECR_Overlap"))))

(fn `UserConstructionScript`)