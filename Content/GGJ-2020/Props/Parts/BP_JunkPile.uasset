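; BP_JunkPile is a damageable junk pile prop that scatters junk pieces when hit.
; The construction script picks the big or regular mesh and sets matching health from the IsBigPile flag.
; Any damage lowers health, prints it on screen and spawns a BP_Junk at a random offset around the mesh.
; When health runs out, the pile spawns a burst of extra junk and destroys itself.
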(event `self.ReceiveAnyDamage`
  (params (Damage :type "Float (single-precision)") (DamageType :type "DamageType Object Reference") (InstigatedBy :type "Controller Object Reference") (DamageCauser :type "Actor Object Reference"))
  (bind _output_get (set `self.Health` (- (`self.Health`) Damage)))
  (`KismetSystemLibrary.PrintString` (`KismetStringLibrary.Conv_DoubleToString` _output_get))
  (`self.SpawnJunk`)
  (if (<= _output_get 0.0)
    (for _ (range 11)
      (`self.SpawnJunk`))
    (`self.K2_DestroyActor`)))

(fn `SpawnJunk`
  (`|SpawnActorFromClass` "/Game/GGJ-2020/Props/Parts/BP_Junk.BP_Junk_C" (`KismetMathLibrary.Conv_VectorToTransform` (+ (* (`KismetMathLibrary.RandomUnitVector`) 50.0) (`SceneComponent.K2_GetComponentLocation` (`self.SM_JunkPile_Big`)))) "AlwaysSpawn" "OverrideRootScale" null null))

(fn `UserConstructionScript`
  (bind _sm_junkpile_big (`self.SM_JunkPile_Big`))
  (if (`self.IsBigPile`)
    (`StaticMeshComponent.SetStaticMesh` _sm_junkpile_big "/Game/GGJ-2020/Props/Parts/SM_JunkPile_Big.SM_JunkPile_Big")
    (set `self.Health` 150.0)
    (else
      (`StaticMeshComponent.SetStaticMesh` _sm_junkpile_big "/Game/GGJ-2020/Props/Parts/SM_JunkPile.SM_JunkPile")
      (set `self.Health` 100.0))))