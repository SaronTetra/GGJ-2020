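; Spanner melee weapon actor that swings on its Attack event and damages what it hits.
; A DoOnce gate blocks new attacks until the timeline-driven relative rotation and offset swing finishes.
; As the swing starts, a single visibility line trace along the mesh's right vector applies point damage on a hit, with separate hit and miss sounds played at world origin.
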(event `Attack`
  (bind _sm_spanner (`self.SM_Spanner`))
  (bind _returnvalue (`SceneComponent.K2_GetComponentLocation` _sm_spanner))
  (`/Engine/EditorBlueprintResources/StandardMacros.DoOnce` false :!label _label
    (:`Completed`
      (`|ExecutionSequence`
        (:`then_0`
          ;[1 1 1] Rotate
          (bind (_direction _rotation) (`Timeline|AttackTimeline` :!via `PlayFromStart`)
            (:`Update`
              (`self.K2_SetActorRelativeRotation` (`KismetMathLibrary.MakeRotator` 0.0 0.0 (* _rotation -45.0)))
              (`self.K2_SetActorRelativeLocation` (`KismetMathLibrary.MakeVector` 0.0 (* _rotation 25.0))))
            (:`Finished`
              (goto _label :!via `Reset`))))
        (:`then_1`
          (bind _outhit (`KismetSystemLibrary.LineTraceSingle` _returnvalue (+ _returnvalue (* (`KismetMathLibrary.GetRightVector` (`SceneComponent.K2_GetComponentRotation` _sm_spanner)) (`self.Range`))) "TraceTypeQuery1"))
          (bind (_bblockinghit _binitialoverlap _time _distance _location _impactpoint _normal _impactnormal _physmat _hitactor) (`GameplayStatics.BreakHitResult` _outhit))
          (if (> _distance 0.0)
            (`GameplayStatics.PlaySoundAtLocation` "/Game/GGJ-2020/Spanner/Crowbar/A_SpannerrHit_Cue.A_SpannerrHit_Cue" (0.0 0.0 0.0) (struct) 1.0 1.0 0.0 null null null)
            (`GameplayStatics.ApplyPointDamage` _hitactor 15.0 _impactpoint _outhit)
            (else
              (`GameplayStatics.PlaySoundAtLocation` "/Game/GGJ-2020/Spanner/Crowbar/A_SpannerMiss_Cue.A_SpannerMiss_Cue" (0.0 0.0 0.0) (struct) 1.0 1.0 0.0 null null null))))))))

(fn `UserConstructionScript`)